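; Player tank Blueprint that provides orbit camera aiming and registers its Barrel component.
; BeginPlay passes Barrel to SetBarrelReference.
; The AimAzimuth and AimElevation axes drive yaw on AzimuthGimbal and pitch on SpringArm separately, as local rotations scaled by delta time and a fixed speed.
; Tick, overlap and construction script are empty.
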(event `self.ReceiveBeginPlay`
  (`self.SetBarrelReference` (`self.Barrel`)))

(event `InputAxis|AimAzimuth`
  (params (AxisValue :type "Float (single-precision)"))
  ;[1 1 1] Camera Input Binding
  (`SceneComponent.K2_AddLocalRotation` (`self.Azimuth Gimbal`) (`KismetMathLibrary.MakeRotator` 0.0 0.0 (* AxisValue (`GameplayStatics.GetWorldDeltaSeconds`) 100.0)) false false))

(event `InputAxis|AimElevation`
  (params (AxisValue :type "Float (single-precision)"))
  ;[1 1 1] Camera Input Binding
  (`SceneComponent.K2_AddLocalRotation` (`self.SpringArm`) (`KismetMathLibrary.MakeRotator` 0.0 (* AxisValue (`GameplayStatics.GetWorldDeltaSeconds`) 100.0)) false false))

(fn `UserConstructionScript`)